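; Game mode for local two-player PVP in which both players control Paladin characters.
; On BeginPlay it creates a second local player, then spawns a Paladin at each PlayerStart, possessed by controller 0 for the first and controller 1 for later ones.
; It then adds a player widget to the player screen for each Paladin found.
; A PauseGame event removes those top-level player widgets without pausing the game itself.
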(event `self.ReceiveBeginPlay`
  (`self.Spawn Players`)
  ;[1 1 1] Adds Widget to screen
  (bind _outactors (`GameplayStatics.GetAllActorsOfClass` "/Game/Blueprints/Character/Player1/MyPlayerCharacter_Paladin.MyPlayerCharacter_Paladin_C"))
  (for _ _outactors
    (bind _returnvalue (`|CreateWidget` "/Game/Blueprints/UI/BP_MyPlayerWidget.BP_MyPlayerWidget_C"))
    (`UserWidget.AddToPlayerScreen` _returnvalue 0)))

(event `Pause Game`
  (bind _foundwidgets (`WidgetBlueprintLibrary.GetAllWidgetsOfClass` "/Game/Blueprints/UI/BP_MyPlayerWidget.BP_MyPlayerWidget_C"))
  (`Widget.RemoveFromParent` _foundwidgets))

(fn `Spawn Players`
  (`GameplayStatics.CreatePlayer` 1)
  ;[1 1 1] Gets players within the game and possesses them
  (bind _outactors (`GameplayStatics.GetAllActorsOfClass` "/Script/Engine.PlayerStart"))
  (for (_array_element _array_index) _outactors
    (if (> _array_index 0)
      (bind _returnvalue (`self.GetTransform` _array_element))
      (bind _returnvalue_2 (`|SpawnActorFromClass` "/Game/Blueprints/Character/Player1/MyPlayerCharacter_Paladin.MyPlayerCharacter_Paladin_C" _returnvalue "Undefined" "MultiplyWithRoot" null null))
      (bind _output_get (set `self.PlayerTwo` _returnvalue_2))
      (`Controller.Possess` (`GameplayStatics.GetPlayerController` 1) _output_get)
      (else
        (bind _returnvalue_3 (`|SpawnActorFromClass` "/Game/Blueprints/Character/Player1/MyPlayerCharacter_Paladin.MyPlayerCharacter_Paladin_C" _returnvalue "Undefined" "MultiplyWithRoot" null null))
        (bind _output_get_2 (set `self.PlayerOne` _returnvalue_3))
        (`Controller.Possess` (`GameplayStatics.GetPlayerController` 0) _output_get_2)))))

(fn `UserConstructionScript`)