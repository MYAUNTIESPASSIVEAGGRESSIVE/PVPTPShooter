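; Pistol weapon that fires hitscan shots and manages magazine and reserve ammo.
; ShootingGun spends a round and line-traces on Visibility from the supplied CameraHolder, with persistent debug drawing, damaging any MyPlayerCharacter_Paladin it hits.
; When one round or fewer remains, it calls Reload instead of firing.
; Reload refills the magazine if any reserve exists, always deducting a full MaxAmmo from the reserve.
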(fn `Reload`
  (bind _maxammo (`self.MaxAmmo`))
  ;[1 1 1] Reload
  (if (> (`self.CurrReserveAmmo`) 0)
    (set `self.CurrAmmo` _maxammo)
    (set `self.CurrReserveAmmo` (- (`self.CurrReserveAmmo`) _maxammo))))

(fn `ShootingGun`
  (params (CameraHolder :type "CameraComponent Object Reference"))
  (bind _returnvalue (`SceneComponent.K2_GetComponentLocation` CameraHolder))
  ;[1 1 1] Trace and Ammo Checks
  (if (<= (`self.CurrAmmo`) 1)
    (`self.Reload`)
    (else
      (set `self.CurrAmmo` (- (`self.CurrAmmo`) 1))
      (bind (_outhit _returnvalue_2) (`KismetSystemLibrary.LineTraceSingle` :`Start` _returnvalue :`End` (+ _returnvalue (* (`KismetMathLibrary.GetForwardVector` (`SceneComponent.K2_GetComponentRotation` CameraHolder)) 3000.0)) :`TraceChannel` "TraceTypeQuery1" :`DrawDebugType` "Persistent" :`TraceColor` (struct :`G` 0.208144 :`B` 1.0 :`A` 1.0)))
      (`KismetSystemLibrary.PrintString` "Hit" _returnvalue_2)
      (bind _asmy_player_character_paladin (cast `/Game/Blueprints/Character/Player1/MyPlayerCharacter_Paladin` (`.HitActor` (`GameplayStatics.BreakHitResult` _outhit))))
      (`/Game/Blueprints/Character/Player1/MyPlayerCharacter_Paladin.Damage` _asmy_player_character_paladin (`KismetMathLibrary.Conv_IntToDouble` (`self.Damage`))))))

(fn `UserConstructionScript`)